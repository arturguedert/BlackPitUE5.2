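; GameState Blueprint that serves as the central UI manager for menus, HUD, pause, end and death screens.
; BeginPlay creates every widget once and caches it, and custom events add or remove them from the viewport.
; Menu, pause, end and death events also switch input mode and cursor visibility, with pause events toggling game pause and the HUD.
; It also stores a Sequence reference that other code can update and stop.
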(event `Update Sequence`
  (params (Sequence :type "MovieSceneSequencePlayer Object Reference"))
  ;[1 1 1] Sequence
  (set `self.Sequence` Sequence))

(event `Stop Sequence`
  ;[1 1 1] Sequence
  (`MovieSceneSequencePlayer.Stop` (`self.Sequence`)))

(event `self.ReceiveBeginPlay`
  (bind _returnvalue (`GameplayStatics.GetPlayerController` 0))
  (bind _returnvalue_2 (`|CreateWidget` "/Game/UI/MainMenu_UI.MainMenu_UI_C" _returnvalue))
  (set `self.MainMenu` _returnvalue_2)
  (bind _returnvalue_3 (`|CreateWidget` "/Game/UI/PauseMenu_UI.PauseMenu_UI_C" _returnvalue))
  (set `self.Pause Menu` _returnvalue_3)
  (bind _returnvalue_4 (`|CreateWidget` "/Game/UI/HUD_UI.HUD_UI_C" _returnvalue))
  (set `self.HUD` _returnvalue_4)
  (bind _returnvalue_5 (`|CreateWidget` "/Game/UI/SettingsPause_UI.SettingsPause_UI_C" _returnvalue))
  (set `self.SettingsPauseMenu` _returnvalue_5)
  (bind _returnvalue_6 (`|CreateWidget` "/Game/UI/SettingsMain_UI.SettingsMain_UI_C" _returnvalue))
  (set `self.SettingsMainMenu` _returnvalue_6)
  (bind _returnvalue_7 (`|CreateWidget` "/Game/UI/End_UI.End_UI_C" _returnvalue))
  (set `self.EndUI` _returnvalue_7)
  (bind _returnvalue_8 (`|CreateWidget` "/Game/UI/Dead_UI.Dead_UI_C" _returnvalue))
  (set `self.DeadUI` _returnvalue_8))

(event `AddHUD`
  ;[1 1 1] HUD
  (`UserWidget.AddToViewport` (`self.HUD`) 0))

(event `RemoveHUD`
  ;[1 1 1] HUD
  (`Widget.RemoveFromParent` (`self.HUD`)))

(event `UnpauseGame`
  (bind _returnvalue (`GameplayStatics.GetPlayerController` 0))
  ;[1 1 1] Pause
  (`GameplayStatics.SetGamePaused` false)
  (`self.AddHUD`)
  (`Widget.RemoveFromParent` (`self.Pause Menu`))
  (`WidgetBlueprintLibrary.SetInputMode_GameOnly` _returnvalue)
  (set `PlayerController.bShowMouseCursor` false _returnvalue))

(event `PauseGame`
  (bind _returnvalue (`GameplayStatics.GetPlayerController` 0))
  ;[1 1 1] Pause
  (`GameplayStatics.SetGamePaused` true)
  (`self.RemoveHUD`)
  (`UserWidget.AddToViewport` (`self.Pause Menu`) 0)
  (`WidgetBlueprintLibrary.SetInputMode_UIOnlyEx` _returnvalue null)
  (set `PlayerController.bShowMouseCursor` true _returnvalue))

(event `Open SettingsPause`
  ;[1 1 1] Settings
  (`UserWidget.AddToViewport` (`self.SettingsPauseMenu`) 0))

(event `OpenSettingsMain`
  ;[1 1 1] Settings
  (`UserWidget.AddToViewport` (`self.SettingsMainMenu`) 0))

(event `Close SettingsPause`
  ;[1 1 1] Settings
  (`Widget.RemoveFromParent` (`self.SettingsPauseMenu`)))

(event `CloseSettingsMain`
  ;[1 1 1] Settings
  (`Widget.RemoveFromParent` (`self.SettingsMainMenu`)))

(event `Close Main Menu`
  (bind _returnvalue (`GameplayStatics.GetPlayerController` 0))
  ;[1 1 1] Main Menu
  (`Widget.RemoveFromParent` (`self.MainMenu`))
  (`WidgetBlueprintLibrary.SetInputMode_GameOnly` _returnvalue)
  (set `PlayerController.bShowMouseCursor` false _returnvalue))

(event `Open Main Menu`
  (bind _returnvalue (`GameplayStatics.GetPlayerController` 0))
  ;[1 1 1] Main Menu
  (`UserWidget.AddToViewport` (`self.MainMenu`) 0)
  (`WidgetBlueprintLibrary.SetInputMode_UIOnlyEx` _returnvalue null)
  (set `PlayerController.bShowMouseCursor` true _returnvalue))

(event `Open End UI`
  (bind _returnvalue (`GameplayStatics.GetPlayerController` 0))
  (`UserWidget.AddToViewport` (`self.EndUI`) 0)
  (`WidgetBlueprintLibrary.SetInputMode_UIOnlyEx` _returnvalue null)
  (set `PlayerController.bShowMouseCursor` true _returnvalue))

(event `Close End UI`
  (bind _returnvalue (`GameplayStatics.GetPlayerController` 0))
  (`Widget.RemoveFromParent` (`self.EndUI`))
  (`WidgetBlueprintLibrary.SetInputMode_GameOnly` _returnvalue)
  (set `PlayerController.bShowMouseCursor` false _returnvalue))

(event `Open Death UI`
  (bind _returnvalue (`GameplayStatics.GetPlayerController` 0))
  (`UserWidget.AddToViewport` (`self.DeadUI`) 0)
  (`WidgetBlueprintLibrary.SetInputMode_UIOnlyEx` _returnvalue null)
  (set `PlayerController.bShowMouseCursor` true _returnvalue))

(fn `UserConstructionScript`)