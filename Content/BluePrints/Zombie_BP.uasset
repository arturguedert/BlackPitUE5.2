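; Zombie enemy character that runs one of two behavior trees and feeds it blackboard state for player sighting, hits, death and attacks.
; Seeing or hearing a pawn starts a faster chase, while damage updates a life bar and triggers a hit reaction or death, which notifies the Paladin player.
; Hand and bite colliders toggled by events damage the Paladin, with resettable DoOnce gates limiting repeat hits.
; Player proximity reveals the life bar.
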(event `self.ReceiveBeginPlay`
  (bind _returnvalue (`AIBlueprintHelperLibrary.GetAIController` self))
  (`AIController.RunBehaviorTree` _returnvalue (select `bool` (`self.FirstZombie`) :`false` "/Game/AI/Zombie_BT.Zombie_BT" :`true` "/Game/AI/FirstZombie_BT.FirstZombie_BT" :!type "BehaviorTree Object Reference"))
  (bind _blackboardcomponent (`AIController.UseBlackboard` _returnvalue "/Game/AI/Zombie_BB.Zombie_BB"))
  (bind _output_get (set `self.Blackboard Component` _blackboardcomponent))
  (`BlackboardComponent.SetValueAsVector` _output_get "TargetLocation" (`self.K2_GetActorLocation` (`GameplayStatics.GetPlayerCharacter` 0)))
  (`BlackboardComponent.SetValueAsInt` _output_get "Attack Index" 0)
  (set `self.CurrentLife` (`self.MaxLife`))
  (bind _asenemy_ui (cast `/Game/UI/Enemy_UI` (`WidgetComponent.GetWidget` (`self.LifeBar_UI`))))
  (set `self.Enemy UI` _asenemy_ui)
  (bind _returnvalue_2 (`GameplayStatics.GetActorOfClass` "/Script/Engine.TriggerVolume"))
  (set `self.Trigger Volume` _returnvalue_2))

(event `self.PawnSensing.OnHearNoise`
  (params (Instigator :type "Pawn Object Reference") (Location :type "Vector Structure (by ref)") (Volume :type "Float (single-precision)"))
  ;[1 1 1] Pawn Seeing
  (bind _output_get (set `self.PlayerSeen` true :!label _label))
  (`BlackboardComponent.SetValueAsBool` (`self.Blackboard Component`) "PlayerSeen" _output_get)
  (set `CharacterMovementComponent.MaxWalkSpeed` (`self.ChasingSpeed`) (`self.CharacterMovement`)))

(event `self.PawnSensing.OnSeePawn`
  (params (Pawn :type "Pawn Object Reference"))
  ;[1 1 1] Pawn Seeing
  (goto _label))

(event `Player Seen`
  ;[1 1 1] Pawn Seeing
  (goto _label))

(event `ResetZombieGetHit`
  ;[1 1 1] Take Damage
  (goto _label_2 :!via `Reset`))

(event `TakeDamage`
  (params (DamageValue :type "Float (double-precision)"))
  ;[1 1 1] Take Damage
  (`/Engine/EditorBlueprintResources/StandardMacros.DoOnce` false :!label _label_2
    (:`Completed`
      (if (> (`self.CurrentLife`) 0.0)
        (bind _output_get (set `self.CurrentLife` (- (`self.CurrentLife`) DamageValue)))
        (`ProgressBar.SetPercent` (`/Game/UI/Enemy_UI.LifeBar` (`self.Enemy UI`)) (/ _output_get (`self.MaxLife`)))
        (bind _output_get_2 (set `self.PlayerSeen` true))
        (`BlackboardComponent.SetValueAsBool` (`self.Blackboard Component`) "PlayerSeen" _output_get_2)
        (if (> (`self.CurrentLife`) 0.0)
          (`self.Hit Reaction`)
          (else
            (`self.Death`)))
        (set `self.Attacking` false)))))

(event `Death`
  ;[1 1 1] Death
  (bind _output_get (set `self.isDead` true))
  (`BlackboardComponent.SetValueAsBool` (`self.Blackboard Component`) "isDead" _output_get)
  (bind _aspaladin_tpc_bp (cast `/Game/BluePrints/Paladin_TPC_BP` (`GameplayStatics.GetPlayerPawn` 0)))
  (`/Game/BluePrints/Paladin_TPC_BP.Update Current Enemies` _aspaladin_tpc_bp)
  (`SceneComponent.SetHiddenInGame` (`self.LifeBar_UI`) true true))

(event `Hit Reaction`
  ;[1 1 1] Hit Reaction
  (bind _output_get (set `self.Hit` true))
  (`BlackboardComponent.SetValueAsBool` (`self.Blackboard Component`) "Hit" _output_get)
  (`KismetSystemLibrary.Delay` 0.2)
  (bind _output_get_2 (set `self.Hit` false))
  (`BlackboardComponent.SetValueAsBool` (`self.Blackboard Component`) "Hit" _output_get_2))

(event `self.Hand_L Collision.OnComponentBeginOverlap`
  (params (OverlappedComponent :type "PrimitiveComponent Object Reference") (OtherActor :type "Actor Object Reference") (OtherComp :type "PrimitiveComponent Object Reference") (OtherBodyIndex :type Integer) (bFromSweep :type Boolean) (SweepResult :type "HitResult Structure (by ref)"))
  ;[1 1 1] Attack
  (bind _aspaladin_tpc_bp (cast `/Game/BluePrints/Paladin_TPC_BP` OtherActor))
  (`/Engine/EditorBlueprintResources/StandardMacros.DoOnce` false :!label _label_3
    (:`Completed`
      (`/Game/BluePrints/Paladin_TPC_BP.Get Hit` _aspaladin_tpc_bp (`self.PunchDamage`) self))))

(event `Start R Collision`
  ;[1 1 1] Attack
  (set `PrimitiveComponent.bGenerateOverlapEvents` true (`self.Hand_R Collision`)))

(event `End R Collision`
  ;[1 1 1] Attack
  (set `PrimitiveComponent.bGenerateOverlapEvents` false (`self.Hand_R Collision`)))

(event `Start L Collision`
  ;[1 1 1] Attack
  (set `PrimitiveComponent.bGenerateOverlapEvents` true (`self.Hand_L Collision`)))

(event `Reset Attack`
  ;[1 1 1] Attack
  (`|ExecutionSequence`
    (:`then_0`
      (goto _label_3 :!via `Reset`))
    (:`then_1`
      (goto _label_4 :!via `Reset`))
    (:`then_2`
      (goto _label_5 :!via `Reset`))))

(event `self.Hand_R Collision.OnComponentBeginOverlap`
  (params (OverlappedComponent :type "PrimitiveComponent Object Reference") (OtherActor :type "Actor Object Reference") (OtherComp :type "PrimitiveComponent Object Reference") (OtherBodyIndex :type Integer) (bFromSweep :type Boolean) (SweepResult :type "HitResult Structure (by ref)"))
  ;[1 1 1] Attack
  (bind _aspaladin_tpc_bp (cast `/Game/BluePrints/Paladin_TPC_BP` OtherActor))
  (`/Engine/EditorBlueprintResources/StandardMacros.DoOnce` false :!label _label_4
    (:`Completed`
      (`/Game/BluePrints/Paladin_TPC_BP.Get Hit` _aspaladin_tpc_bp (`self.PunchDamage`) self))))

(event `End L Collision`
  ;[1 1 1] Attack
  (set `PrimitiveComponent.bGenerateOverlapEvents` false (`self.Hand_L Collision`)))

(event `Start Bite Collision`
  ;[1 1 1] Attack
  (set `PrimitiveComponent.bGenerateOverlapEvents` true (`self.Bite Collision`)))

(event `self.Bite Collision.OnComponentBeginOverlap`
  (params (OverlappedComponent :type "PrimitiveComponent Object Reference") (OtherActor :type "Actor Object Reference") (OtherComp :type "PrimitiveComponent Object Reference") (OtherBodyIndex :type Integer) (bFromSweep :type Boolean) (SweepResult :type "HitResult Structure (by ref)"))
  ;[1 1 1] Attack
  (bind _aspaladin_tpc_bp (cast `/Game/BluePrints/Paladin_TPC_BP` OtherActor))
  (`/Engine/EditorBlueprintResources/StandardMacros.DoOnce` false :!label _label_5
    (:`Completed`
      (`/Game/BluePrints/Paladin_TPC_BP.Get Hit` _aspaladin_tpc_bp (`self.BiteDamage`) self))))

(event `End Bite Collision`
  ;[1 1 1] Attack
  (set `PrimitiveComponent.bGenerateOverlapEvents` false (`self.Bite Collision`)))

(event `DrawUI`
  (`SceneComponent.SetVisibility` (`self.LifeBar_UI`) true false))

(event `RemoveUI`
  (`SceneComponent.SetVisibility` (`self.LifeBar_UI`) false false))

(event `self.DrawUI Collision.OnComponentBeginOverlap`
  (params (OverlappedComponent :type "PrimitiveComponent Object Reference") (OtherActor :type "Actor Object Reference") (OtherComp :type "PrimitiveComponent Object Reference") (OtherBodyIndex :type Integer) (bFromSweep :type Boolean) (SweepResult :type "HitResult Structure (by ref)"))
  (bind _aspaladin_tpc_bp (cast `/Game/BluePrints/Paladin_TPC_BP` OtherActor))
  (if (not (`/Game/BluePrints/Paladin_TPC_BP.isDead` _aspaladin_tpc_bp))
    (`self.DrawUI`)))

(fn `UserConstructionScript`)