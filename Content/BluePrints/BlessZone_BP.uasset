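; BlessZone_BP is a trigger zone that lets the paladin player bless once their quest index reaches at least 2.
; Entering the capsule shows BlessUI and sets the player's CanBless flag, gated by a DoOnce.
; Leaving hides the UI, clears the flag and resets the DoOnce.
; A separate HideUI event also hides the prompt without changing the flag.
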(event `self.Capsule.OnComponentBeginOverlap`
  (params (OverlappedComponent :type "PrimitiveComponent Object Reference") (OtherActor :type "Actor Object Reference") (OtherComp :type "PrimitiveComponent Object Reference") (OtherBodyIndex :type Integer) (bFromSweep :type Boolean) (SweepResult :type "HitResult Structure (by ref)"))
  (bind _aspaladin_tpc_bp (cast `/Game/BluePrints/Paladin_TPC_BP` OtherActor))
  (bind _output_get (set `self.Player` _aspaladin_tpc_bp))
  (if (>= (`/Game/BluePrints/Paladin_TPC_BP.Quest Index` _output_get) 2)
    (`/Engine/EditorBlueprintResources/StandardMacros.DoOnce` false :!label _label
      (:`Completed`
        (`SceneComponent.SetVisibility` (`self.Bless UI`) true false)
        (set `/Game/BluePrints/Paladin_TPC_BP.CanBless` true (`self.Player`))))))

(event `self.Capsule.OnComponentEndOverlap`
  (params (OverlappedComponent :type "PrimitiveComponent Object Reference") (OtherActor :type "Actor Object Reference") (OtherComp :type "PrimitiveComponent Object Reference") (OtherBodyIndex :type Integer))
  (bind _aspaladin_tpc_bp (cast `/Game/BluePrints/Paladin_TPC_BP` OtherActor))
  (`SceneComponent.SetVisibility` (`self.Bless UI`) false false)
  (set `/Game/BluePrints/Paladin_TPC_BP.CanBless` false _aspaladin_tpc_bp)
  (goto _label :!via `Reset`))

(event `Hide UI`
  (`SceneComponent.SetVisibility` (`self.Bless UI`) false false))

(fn `UserConstructionScript`)